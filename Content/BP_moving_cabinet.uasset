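; BP_moving_cabinet is an actor, named as a cabinet, that slides in a straight line and removes itself.
; BeginPlay stores the spawn point's distance from the world origin as DespawnDistance.
; Tick moves it along world negative X at MoveSpeed scaled by delta time, without sweep, ignoring its own rotation.
; It destroys itself once farther from the origin than it spawned, allowing a pass across the origin's vicinity.
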(event EventBeginPlay
  (bind _output_get (Variables|Default|SetSpawnLocation (Transformation|GetActorLocation)))
  (Variables|Default|SetDespawnDistance (Math|Vector|VectorLength _output_get)))

(event EventActorBeginOverlap
  (params (OtherActor :type Actor%20Object%20Reference)))

(event EventTick
  (params (DeltaSeconds :type Float%20%28single-precision%29))
  (Transformation|SetActorLocation (- (Transformation|GetActorLocation) (* (* (Math|Vector|GetForwardVector "0, 0, 0") (Variables|Default|GetMoveSpeed)) DeltaSeconds)) false false)
  (if (> (Math|Vector|VectorLength (Transformation|GetActorLocation)) (Variables|Default|GetDespawnDistance))
    (Actor|DestroyActor)))

(fn ConstructionScript)