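; BP_moving_cabinet is a cabinet actor that slides in a straight line along world negative X at MoveSpeed.
; BeginPlay stores the spawn point's distance from the world origin as the despawn threshold.
; Tick moves it without sweep and destroys it once it is farther from the origin than that threshold.
; The Hit event only prints a debug "Hello".
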(event EventBeginPlay
  (bind _output_get (Variables|Default|SetSpawnLocation (Transformation|GetActorLocation)))
  (Variables|Default|SetDespawnDistance (Math|Vector|VectorLength _output_get)))

(event EventActorBeginOverlap
  (params (OtherActor :type Actor%20Object%20Reference)))

(event EventTick
  (params (DeltaSeconds :type Float%20%28single-precision%29))
  (Transformation|SetActorLocation (- (Transformation|GetActorLocation) (* (* (Math|Vector|GetForwardVector "0, 0, 0") (Variables|Default|GetMoveSpeed)) DeltaSeconds)) false false)
  (if (> (Math|Vector|VectorLength (Transformation|GetActorLocation)) (Variables|Default|GetDespawnDistance))
    (Actor|DestroyActor)))

(event Collision|EventHit
  (params (MyComp :type Primitive%20Component%20Object%20Reference) (Other :type Actor%20Object%20Reference) (OtherComp :type Primitive%20Component%20Object%20Reference) (bSelfMoved :type Boolean) (HitLocation :type Vector :default "0, 0, 0") (HitNormal :type Vector :default "0, 0, 0") (NormalImpulse :type Vector :default "0, 0, 0") (Hit :type Hit%20Result%20Structure%20%28by%20ref%29))
  (Development|PrintString "Hello"))

(fn ConstructionScript)